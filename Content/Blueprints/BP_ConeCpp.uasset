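; BP_ConeCpp is an actor Blueprint that exercises ways of exposing C++ functions to Blueprints.
; The implementable event TestImplementableFunc forwards its value to TestFunc, while TestImplementableFuncRetVal is a function returning its input.
; A BlueprintNativeEvent example spawns an emitter at the actor, waits briefly, then calls the parent Explode implementation.
; BeginPlay is empty, and sample calls testing pure functions and input/output parameters remain disconnected.
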(event `self.ReceiveBeginPlay`
  ;[0 0.3006 1] TestFunc BlueprintCallable
)

(event `self.TestImplementableFunc`
  (params (Val :type Integer))
  ;[0.1638 0.1602 1] Blueprint Implementable Event (Si genera partendo dalla Tab a sinistra delle funzioni, menu a tendina override e si sceglie TestImplementableFunc e aggiungere nel CPP la chiamata a funzione nell'EventBeginPlay). Se la funzione ha un valore di ritorno diventa una funzione Blueprint
  (`self.TestFunc` Val))

(event `CustomEvent`
  ;[0 0.07604 1] BlueprintNativeEvent (si dichiara la funzione in CPP ma non si implementa ma si implementa una funzione che termina con _Implementation; cliccare sull'evento e generare il parent)
  (`GameplayStatics.SpawnEmitterAtLocation` null (`self.K2_GetActorLocation`))
  (`KismetSystemLibrary.Delay` 0.2)
  (`parent.Explode`))

(fn `TestImplementableFuncRetVal`
  (params (Val :type Integer))
  (returns (ReturnValue :type Integer))
  (return Val))

(fn `UserConstructionScript`)