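; BP_ConeBP is an actor that moves continuously up and down between its starting height and a Max offset above it.
; BeginPlay records the start Z as the lower bound and derives the upper bound from Max.
; Tick shifts Z by Speed scaled by delta time, sets the location without sweep, and flips the IsUp flag once a bound is passed.
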(event `self.ReceiveBeginPlay`
  (bind (_returnvalue_x _returnvalue_y _returnvalue_z) (`KismetMathLibrary.BreakVector` (`self.K2_GetActorLocation`)))
  (set `self.bIsUp` true)
  (set `self.CurrentZ` _returnvalue_z)
  (set `self.MinHeight` _returnvalue_z)
  (set `self.MaxHeight` (+ _returnvalue_z (`self.Max`))))

(event `self.ReceiveTick`
  (params (DeltaSeconds :type "Float (single-precision)"))
  (bind (_returnvalue_x _returnvalue_y) (`KismetMathLibrary.BreakVector` (`self.K2_GetActorLocation`)))
  (bind _returnvalue (* DeltaSeconds (`self.Speed`)))
  (if (`self.bIsUp`)
    (set `self.CurrentZ` (+ (`self.CurrentZ`) _returnvalue))
    (else
      (set `self.CurrentZ` (- (`self.CurrentZ`) _returnvalue))))
  (`self.K2_SetActorLocation` (`KismetMathLibrary.MakeVector` _returnvalue_x _returnvalue_y (`self.CurrentZ`)))
  (if (> (`self.CurrentZ`) (`self.MaxHeight`))
    (set `self.bIsUp` false))
  (if (< (`self.CurrentZ`) (`self.MinHeight`))
    (set `self.bIsUp` true)))

(fn `UserConstructionScript`)